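; Infinite-style ocean surface actor built as a clipmap of procedural plane sections.
; Construction generates a dense centre grid and rings doubling in size per LOD, each section with a dynamic material carrying LOD index and color.
; Each tick it scales in power-of-two steps with camera height and snaps XY to the camera on a scale-relative grid.
; Scale, quad count, section size and snapped position feed MPC_OceanSimulation for shaders.
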(event `self.ReceiveTick`
  (params (DeltaSeconds :type "Float (single-precision)"))
  (bind (_returnvalue_x _returnvalue_y _returnvalue_z) (`KismetMathLibrary.BreakVector` (`self.K2_GetActorLocation`)))
  (bind (_returnvalue_x_2 _returnvalue_y_2) (`KismetMathLibrary.BreakVector` (`self.K2_GetActorLocation` (`GameplayStatics.GetPlayerCameraManager` 0))))
  (bind (_returnvalue_x_3 _returnvalue_y_3 _returnvalue_z_2) (`KismetMathLibrary.BreakVector` (`self.K2_GetActorLocation` (`GameplayStatics.GetPlayerCameraManager` 0))))
  (bind _returnvalue (* (`self.Scale`) 25.0))
  (bind _returnvalue_2 (/ _returnvalue_y_2 _returnvalue))
  (bind _returnvalue_3 (/ _returnvalue_x_2 _returnvalue))
  (bind _returnvalue_4 (`KismetMathLibrary.MakeVector` (* (`KismetMathLibrary.SelectFloat` (`KismetMathLibrary.Conv_IntToDouble` (`KismetMathLibrary.FCeil` _returnvalue_3)) (`KismetMathLibrary.Conv_IntToDouble` (`KismetMathLibrary.FFloor` _returnvalue_3)) (>= _returnvalue_x_2 0.0)) _returnvalue) (* (`KismetMathLibrary.SelectFloat` (`KismetMathLibrary.Conv_IntToDouble` (`KismetMathLibrary.FFloor` _returnvalue_2)) (`KismetMathLibrary.Conv_IntToDouble` (`KismetMathLibrary.FCeil` _returnvalue_2)) (>= _returnvalue_y_2 0.0)) _returnvalue) _returnvalue_z))
  (`|ExecutionSequence`
    (:`then_0`
      (bind _output_get (set `self.Height` _returnvalue_z_2))
      (if (> _returnvalue_z_2 64.0)
        (bind _output_get_2 (set `self.HeightLog` (`KismetMathLibrary.Log` _output_get 2.0)))
        (bind _output_get_3 (set `self.Scale` (`KismetMathLibrary.FMax` (/ (* (`KismetMathLibrary.MultiplyMultiply_FloatFloat` 2.0 (`KismetMathLibrary.Conv_IntToDouble` (`KismetMathLibrary.FFloor` _output_get_2))) 0.5) 32.0) 1.0)))
        (`self.SetActorScale3D` (`KismetMathLibrary.Conv_DoubleToVector` _output_get_3))))
    (:`then_1`
      (`self.K2_SetActorLocation` _returnvalue_4)
      (`KismetMaterialLibrary.SetVectorParameterValue` "/InfinityEnvironment/InfinityOcean/Ocean/OceanData/MPC_OceanSimulation.MPC_OceanSimulation" "OceanMesh_CameraPos" (`KismetMathLibrary.Conv_VectorToLinearColor` _returnvalue_4)))
    (:`then_2`
      (`self.UpdateShaderResource`))))

(fn `UpdateShaderResource`
  (`KismetMaterialLibrary.SetScalarParameterValue` "/InfinityEnvironment/InfinityOcean/Ocean/OceanData/MPC_OceanSimulation.MPC_OceanSimulation" "OceanMesh_Scale" (`self.Scale`))
  (`KismetMaterialLibrary.SetScalarParameterValue` "/InfinityEnvironment/InfinityOcean/Ocean/OceanData/MPC_OceanSimulation.MPC_OceanSimulation" "OceanMesh_NumQuad" (`KismetMathLibrary.Conv_IntToDouble` (* (`self.NumQuad`) 2)))
  (`KismetMaterialLibrary.SetScalarParameterValue` "/InfinityEnvironment/InfinityOcean/Ocean/OceanData/MPC_OceanSimulation.MPC_OceanSimulation" "OceanMesh_SectionScale" (* (`KismetMathLibrary.Conv_IntToDouble` (* (`self.SectionScale`) (`KismetMathLibrary.FFloor` (`self.Scale`)))) 200.0)))

(fn `UserConstructionScript`
  (bind _sectionscale (`self.SectionScale`))
  (`ProceduralMeshComponent.ClearAllMeshSections` (`self.OceanMesh`))
  (for _index (range 1 (+ (`self.NumLOD`) 1))
    (if (== _index 1)
      (for (_array_element _array_index) (`self.LOD0 Offsets`)
        (bind (_indexarray _uvarray _vertexarray) (`OceanUtillity.GeneratePlaneMesh` true (`self.FlipEdge`) (`self.NumQuad`) (`KismetMathLibrary.Conv_IntToDouble` _sectionscale) (* _array_element _sectionscale)))
        (`ProceduralMeshComponent.CreateMeshSection_LinearColor` :`self` (`self.OceanMesh`) :`SectionIndex` _array_index :`Vertices` _vertexarray :`Triangles` _indexarray :`UV0` _uvarray)
        (bind _returnvalue (`KismetMaterialLibrary.CreateDynamicMaterialInstance` (`self.BaseMaterial`)))
        (bind _returnvalue_2 (- _index 1))
        (bind _returnvalue_3 (`KismetMathLibrary.Conv_IntToDouble` _returnvalue_2))
        (`MaterialInstanceDynamic.SetScalarParameterValue` _returnvalue "LODIndex" _returnvalue_3)
        (bind _output (`|GetArrayItem` (`self.LODColor`) _returnvalue_2))
        (`MaterialInstanceDynamic.SetVectorParameterValue` _returnvalue "LODColor" _output)
        (`PrimitiveComponent.SetMaterial` (`self.OceanMesh`) _array_index _returnvalue))
      (else
        (for (_array_element_2 _array_index_2) (`self.LOD1 Offsets`)
          (bind _returnvalue_4 (- _index 2))
          (bind _returnvalue_5 (* (`self.SectionScale`) (select `int` _returnvalue_4 :`0` 1 :`1` 2 :`2` 4 :`3` 8 :`4` 16 :`5` 32 :`6` 64 :`7` 128 :`8` 256 :`9` 512)))
          (bind (_indexarray_2 _uvarray_2 _vertexarray_2) (`OceanUtillity.GeneratePlaneMesh` true (`self.FlipEdge`) (`self.NumQuad`) (`KismetMathLibrary.Conv_IntToDouble` (* _returnvalue_5 2)) (* _array_element_2 _returnvalue_5)))
          (bind _returnvalue_6 (+ _array_index_2 16 (* 12 _returnvalue_4)))
          (`ProceduralMeshComponent.CreateMeshSection_LinearColor` :`self` (`self.OceanMesh`) :`SectionIndex` _returnvalue_6 :`Vertices` _vertexarray_2 :`Triangles` _indexarray_2 :`UV0` _uvarray_2)
          (bind _returnvalue_7 (`KismetMaterialLibrary.CreateDynamicMaterialInstance` (`self.BaseMaterial`)))
          (`MaterialInstanceDynamic.SetScalarParameterValue` _returnvalue_7 "LODIndex" _returnvalue_3)
          (`MaterialInstanceDynamic.SetVectorParameterValue` _returnvalue_7 "LODColor" _output)
          (`PrimitiveComponent.SetMaterial` (`self.OceanMesh`) _returnvalue_6 _returnvalue_7)))))
  (`self.UpdateShaderResource`))