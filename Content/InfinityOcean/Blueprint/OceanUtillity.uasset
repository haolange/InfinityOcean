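; OceanUtillity provides GenerateOceanBatch, which builds a tiled ocean surface as concentric LOD levels on a supplied procedural mesh component.
; Each tile is a GeneratePlaneMesh grid, placed by the LOD0 or LOD1 offset array and assigned MI_OceanBase.
; Outer levels reuse the LOD1 offsets at power-of-two scales, halving vertex density per level.
; Section indices reserve 16 slots for LOD0 and 12 per outer level.
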(fn `GenerateOceanBatch`
  (params (FlipEdge :type Boolean) (NumLOD :type Integer) (NumQuad :type Integer) (SectionScale :type Integer) (`LOD0 Offsets` :type "Array of Vector Structure") (`LOD1 Offsets` :type "Array of Vector Structure") (MeshComponent :type "ProceduralMeshComponent Object Reference"))
  (for _index (range 1 (+ NumLOD 1))
    (if (== _index 1)
      (for (_array_element _array_index) `LOD0 Offsets`
        (bind (_indexarray _uvarray _vertexarray) (`OceanUtillity.GeneratePlaneMesh` true FlipEdge NumQuad (`KismetMathLibrary.Conv_IntToDouble` SectionScale) (* _array_element SectionScale)))
        (`ProceduralMeshComponent.CreateMeshSection_LinearColor` :`self` MeshComponent :`SectionIndex` _array_index :`Vertices` _vertexarray :`Triangles` _indexarray :`UV0` _uvarray)
        (`PrimitiveComponent.SetMaterial` MeshComponent _array_index "/InfinityEnvironment/InfinityOcean/Ocean/Material/MI_OceanBase.MI_OceanBase"))
      (else
        (for (_array_element_2 _array_index_2) `LOD1 Offsets`
          (bind _returnvalue (- _index 2))
          (bind _returnvalue_2 (* SectionScale (select `int` _returnvalue :`0` 1 :`1` 2 :`2` 4 :`3` 8 :`4` 16 :`5` 32 :`6` 64 :`7` 128 :`8` 256 :`9` 512)))
          (bind (_indexarray_2 _uvarray_2 _vertexarray_2) (`OceanUtillity.GeneratePlaneMesh` true FlipEdge NumQuad (`KismetMathLibrary.Conv_IntToDouble` (* _returnvalue_2 2)) (* _array_element_2 _returnvalue_2)))
          (bind _returnvalue_3 (+ _array_index_2 16 (* 12 _returnvalue)))
          (`ProceduralMeshComponent.CreateMeshSection_LinearColor` :`self` MeshComponent :`SectionIndex` _returnvalue_3 :`Vertices` _vertexarray_2 :`Triangles` _indexarray_2 :`UV0` _uvarray_2)
          (`PrimitiveComponent.SetMaterial` MeshComponent _returnvalue_3 "/InfinityEnvironment/InfinityOcean/Ocean/Material/MI_OceanBase.MI_OceanBase")))))
  (return))